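; AI controller for the BumBI helicopter chaser enemy that flies it toward a target pawn.
; On possess it caches the helicopter, and a SetTargetPlayer event supplies the target.
; Each tick, while both are valid, it calls the helicopter's MoveTowards along the look-at direction to the target, steering directly without navigation pathfinding.
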(event `self.ReceivePossess`
  (params (PossessedPawn :type "Pawn Object Reference"))
  (bind _asbp_enemy_bum_biheli_chaser (cast `/Game/Blueprints/Characters/Enemies/BP_Enemy_BumBIHeli_chaser` PossessedPawn))
  (set `self.OwningBumbiHeli` _asbp_enemy_bum_biheli_chaser))

(event `self.ReceiveTick`
  (params (DeltaSeconds :type "Float (single-precision)"))
  (`/Engine/EditorBlueprintResources/StandardMacros.IsValid` (`self.OwningBumbiHeli`)
    (:`Is Valid`
      (`/Engine/EditorBlueprintResources/StandardMacros.IsValid` (`self.TargetPawn`)
        (:`Is Valid`
          (`/Game/Blueprints/Characters/Enemies/BP_Enemy_BumBIHeli_chaser.MoveTowards` (`self.OwningBumbiHeli`) (`KismetMathLibrary.GetForwardVector` (`KismetMathLibrary.FindLookAtRotation` (`self.K2_GetActorLocation` (`self.OwningBumbiHeli`)) (`self.K2_GetActorLocation` (`self.TargetPawn`)))) 1.0))))))

(event `SetTargetPlayer`
  (params (TargetPawn :type "Pawn Object Reference"))
  (set `self.TargetPawn` TargetPawn))

(fn `UserConstructionScript`
  (`parent.UserConstructionScript`))