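; AI controller for the boss enemy that chases a target pawn and fires fireballs at it on a timer.
; On possessing a BP_Enemy_Boss it caches the boss and starts a looping timer at the shoot interval, with ShootProjectile calling the boss's ShootFireball.
; Each tick it moves the boss straight toward the target set through SetTargetPlayer, using a look-at direction with no navmesh pathfinding.
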(event `self.ReceivePossess`
  (params (PossessedPawn :type "Pawn Object Reference"))
  (bind _asbp_enemy_boss (cast `/Game/Blueprints/Characters/Enemies/Boss/BP_Enemy_Boss` PossessedPawn))
  (set `self.OwningBoss` _asbp_enemy_boss)
  (`KismetSystemLibrary.K2_SetTimerDelegate` (`|CreateDelegate` :!event `ShootProjectile`) (`self.ShootInterval`) true))

(event `ShootProjectile`
  (`/Game/Blueprints/Characters/Enemies/Boss/BP_Enemy_Boss.ShootFireball` (`self.OwningBoss`)))

(event `self.ReceiveTick`
  (params (DeltaSeconds :type "Float (single-precision)"))
  (`/Engine/EditorBlueprintResources/StandardMacros.IsValid` (`self.OwningBoss`)
    (:`Is Valid`
      (`/Engine/EditorBlueprintResources/StandardMacros.IsValid` (`self.TargetPawn`)
        (:`Is Valid`
          (`/Game/Blueprints/Characters/Enemies/Boss/BP_Enemy_Boss.MoveTowards` (`self.OwningBoss`) (`KismetMathLibrary.GetForwardVector` (`KismetMathLibrary.FindLookAtRotation` (`self.K2_GetActorLocation` (`self.OwningBoss`)) (`self.K2_GetActorLocation` (`self.TargetPawn`)))) 1.0))))))

(event `SetTargetPlayer`
  (params (TargetPawn :type "Pawn Object Reference"))
  (set `self.TargetPawn` TargetPawn))

(fn `UserConstructionScript`
  (`parent.UserConstructionScript`))