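; BlasterBeak enemy character that plays a shoot animation and fires its own projectile type.
; ShootFireball plays the Shoot sequence as an override on the animation component's anim instance.
; SpawnProjectile is a separate function that always spawns a BlasterBeak projectile at the ShootPos transform and plays a shot sound at the actor.
; The file defines no active event logic and does not show what calls either function.
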(fn `ShootFireball`
  (`PaperZDAnimInstance.K2_PlayAnimationOverride` (`PaperZDAnimationComponent.AnimInstance` (`self.AnimationComponent`)) "/Game/Blueprints/Characters/Enemies/BlasterBeak/AnimSequences/Shoot.Shoot" "DefaultSlot" 1.0 0.0))

(fn `SpawnProjectile`
  (bind _shootpos (`self.ShootPos`))
  (`|SpawnActorFromClass` "/Game/Blueprints/Projectiles/Enemy/BP_EnemyProjectile_BlasterBeak.BP_EnemyProjectile_BlasterBeak_C" (`KismetMathLibrary.MakeTransform` (`SceneComponent.K2_GetComponentLocation` _shootpos) (`SceneComponent.K2_GetComponentRotation` _shootpos)) "AlwaysSpawn" "MultiplyWithRoot" null null)
  (`GameplayStatics.PlaySoundAtLocation` "/Game/Audio/SFX/Shoot_Lizard_Cue.Shoot_Lizard_Cue" (`self.K2_GetActorLocation`) (struct) 1.0 1.0 0.0 null null null null))

(fn `UserConstructionScript`
  (`parent.UserConstructionScript`))